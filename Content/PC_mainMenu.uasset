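; Main menu player controller that shows the mouse cursor and adds the WB_MainMenu widget to the viewport on BeginPlay.
; It also provides client and server events for hosting a game.
; Client_HostGame forwards to the server host call, and Server_HostGame asks MyGameInstance to host, passing this controller and a map name.
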(event `self.ReceiveBeginPlay`
  (set `self.bShowMouseCursor` true)
  (bind _returnvalue (`|CreateWidget` "/Game/WB_MainMenu.WB_MainMenu_C" self))
  (`UserWidget.AddToViewport` _returnvalue 0))

(event `Client_HostGame`
  (`self.Server_HostGame`))

(event `Server_HostGame`
  (bind _asmy_game_instance (cast `/Game/MyGameInstance` (`GameplayStatics.GetGameInstance`)))
  (`/Game/MyGameInstance.Host` _asmy_game_instance self (`self.MapName`)))

(fn `UserConstructionScript`)