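; Multiplayer test version of a torque-rolled ball pawn, with ball physics disabled on clients and simulated packet lag and loss set at BeginPlay.
; Movement axes apply torque locally and also pass input to server events that apply it with authority.
; On Tick the server sends transform and time to ClientSmoothTransform, meant to trim the client's recorded transform history.
; The buffered interpolation and snapping logic is disconnected, so received transforms are never applied.
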(event `self.ReceiveBeginPlay`
  ;[1 1 1] Make sure the client isn't doing physics, only the server
  (`|ExecutionSequence`
    (:`then_0`
      (`KismetSystemLibrary.ExecuteConsoleCommand` "net pktlag=60" null)
      (`KismetSystemLibrary.ExecuteConsoleCommand` "net pktloss=1" null))
    (:`then_1`
      (`/Engine/EditorBlueprintResources/ActorMacros.Switch Has Authority`
        (:`Remote`
          (`PrimitiveComponent.SetSimulatePhysics` (`self.Ball`) false))))))

(event `ServerMoveForward`
  (params (Value :type "Float (double-precision)"))
  ;[1 1 1] Server-side movement and rotation
  (`/Engine/EditorBlueprintResources/ActorMacros.Switch Has Authority`
    (:`Authority`
      (`PrimitiveComponent.AddTorqueInRadians` (`self.Ball`) (`KismetMathLibrary.MakeVector` 0.0 (* Value (`self.RollTorque`))) "None" false))))

(event `InputAxis|MoveRight`
  (params (AxisValue :type "Float (single-precision)"))
  ;[1 1 1] Roll left/right
  (`PrimitiveComponent.AddTorqueInRadians` (`self.Ball`) (`KismetMathLibrary.MakeVector` (* (`self.RollTorque`) AxisValue -1.0)) "None" false))

(event `ServerMoveRight`
  (params (Value :type "Float (double-precision)"))
  ;[1 1 1] Server-side movement and rotation
  (`/Engine/EditorBlueprintResources/ActorMacros.Switch Has Authority`
    (:`Authority`
      (`PrimitiveComponent.AddTorqueInRadians` (`self.Ball`) (`KismetMathLibrary.MakeVector` (* Value (`self.RollTorque`) -1.0)) "None" false))))

(event `InputAxis|MoveForward`
  (params (AxisValue :type "Float (single-precision)"))
  ;[1 1 1] Replicate movement inputs from client to server
  (if (!= AxisValue 0.0)
    (`self.ServerMoveForward` AxisValue)))

(event `InputAxis|MoveRight`
  (params (AxisValue :type "Float (single-precision)"))
  ;[1 1 1] Replicate movement inputs from client to server
  (if (!= AxisValue 0.0)
    (`self.ServerMoveRight` AxisValue)))

(event `InputAxis|MoveForward`
  (params (AxisValue :type "Float (single-precision)"))
  ;[1 1 1] Roll forwards/backwards
  (`PrimitiveComponent.AddTorqueInRadians` (`self.Ball`) (`KismetMathLibrary.MakeVector` 0.0 (* (`self.RollTorque`) AxisValue)) "None" false))

(event `ClientSmoothTransform`
  (params (Transform :type "Transform Structure") (Time :type "Float (double-precision)"))
  (bind _pastlocationstimes (`self.PastLocationsTimes`))
  (if (not (< (- Time (`|GetArrayItem` _pastlocationstimes)) 0.0)) :!label _label
    (`KismetArrayLibrary.Array_RemoveItem` _pastlocationstimes)
    (`KismetArrayLibrary.Array_RemoveItem` (`self.PastLocations`))
    (goto _label)))

(event `self.ReceiveTick`
  (params (DeltaSeconds :type "Float (single-precision)"))
  ;[1 1 1] Replicate Physics based Movement from server to the owning client
  (`/Engine/EditorBlueprintResources/ActorMacros.Switch Has Authority`
    (:`Authority`
      (`self.ClientSmoothTransform` (`self.GetTransform`) (`GameplayStatics.GetTimeSeconds`)))
    (:`Remote`
      (`KismetArrayLibrary.Array_Add` (`self.PastLocations`) (`self.GetTransform`))
      (`KismetArrayLibrary.Array_Add` (`self.PastLocationsTimes`) (`GameplayStatics.GetTimeSeconds`)))))

(fn `UserConstructionScript`)