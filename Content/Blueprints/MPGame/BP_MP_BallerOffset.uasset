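; Multiplayer rolling-ball pawn with server-authoritative physics and a test of client-side snapshot interpolation under simulated packet lag and loss.
; Move inputs add torque locally and through server events, while remote copies disable physics simulation.
; The server sends timestamped transforms every tick, which remotes buffer and lerp by tick count with a small X offset and zeroed rotation.
; Overfull buffers are periodically skimmed to the newest snapshots, with debug prints throughout.
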(event `self.ReceiveBeginPlay`
  ;[1 1 1] Make sure the client isn't doing physics, only the server
  (`|ExecutionSequence`
    (:`then_0`
      (`KismetSystemLibrary.ExecuteConsoleCommand` "net pktlag=60" null)
      (`KismetSystemLibrary.ExecuteConsoleCommand` "net pktloss=1" null))
    (:`then_1`
      (`/Engine/EditorBlueprintResources/ActorMacros.Switch Has Authority`
        (:`Remote`
          (`PrimitiveComponent.SetSimulatePhysics` (`self.Ball`) false))))))

(event `InputAxis|MoveRight`
  (params (AxisValue :type "Float (single-precision)"))
  ;[1 1 1] Roll left/right
  (`PrimitiveComponent.AddTorqueInRadians` (`self.Ball`) (`KismetMathLibrary.MakeVector` (* (`self.RollTorque`) AxisValue -1.0)) "None" false))

(event `ServerMoveForward`
  (params (Value :type "Float (double-precision)"))
  ;[1 1 1] Server-side movement and rotation
  (`/Engine/EditorBlueprintResources/ActorMacros.Switch Has Authority`
    (:`Authority`
      (`PrimitiveComponent.AddTorqueInRadians` (`self.Ball`) (`KismetMathLibrary.MakeVector` 0.0 (* Value (`self.RollTorque`))) "None" false))))

(event `ServerMoveRight`
  (params (Value :type "Float (double-precision)"))
  ;[1 1 1] Server-side movement and rotation
  (`/Engine/EditorBlueprintResources/ActorMacros.Switch Has Authority`
    (:`Authority`
      (`PrimitiveComponent.AddTorqueInRadians` (`self.Ball`) (`KismetMathLibrary.MakeVector` (* Value (`self.RollTorque`) -1.0)) "None" false))))

(event `InputAxis|MoveForward`
  (params (AxisValue :type "Float (single-precision)"))
  ;[1 1 1] Replicate movement inputs from client to server
  (if (!= AxisValue 0.0)
    (`self.ServerMoveForward` AxisValue)))

(event `InputAxis|MoveForward`
  (params (AxisValue :type "Float (single-precision)"))
  ;[1 1 1] Roll forwards/backwards
  (`PrimitiveComponent.AddTorqueInRadians` (`self.Ball`) (`KismetMathLibrary.MakeVector` 0.0 (* (`self.RollTorque`) AxisValue)) "None" false))

(event `InputAxis|MoveRight`
  (params (AxisValue :type "Float (single-precision)"))
  ;[1 1 1] Replicate movement inputs from client to server
  (if (!= AxisValue 0.0)
    (`self.ServerMoveRight` AxisValue)))

(event `ClientSmoothTransform`
  (params (Transform :type "Transform Structure") (Time :type "Float (double-precision)"))
  (if (and true (> Time (`self.RecentUpdate`)))
    (`KismetArrayLibrary.Array_Add` (`self.Transforms`) Transform)
    (`KismetArrayLibrary.Array_Add` (`self.Times`) Time)
    (set `self.RecentUpdate` Time)
    (`/Engine/EditorBlueprintResources/ActorMacros.Switch Has Authority`
      (:`Remote`
        (bind _outactors (`GameplayStatics.GetAllActorsOfClass` "/Game/Sphere2_Blueprint.Sphere2_Blueprint_C"))))))

(event `self.ReceiveTick`
  (params (DeltaSeconds :type "Float (single-precision)"))
  (bind _times (`self.Times`))
  (bind _interpticksneeded (`self.InterpTicksNeeded`))
  (bind _transforms (`self.Transforms`))
  (bind _times_2 (`self.Times`))
  (bind _returnvalue (`KismetArrayLibrary.Array_Length` _transforms))
  (bind _returnvalue_2 (`KismetMathLibrary.Round` (/ (- (`|GetArrayItem` _times_2 1) (`|GetArrayItem` _times_2)) (`self.deltaSeconds`))))
  (bind _returnvalue_3 (- _returnvalue_2 (`self.TicksSpentInterpolating`)))
  (`/Engine/EditorBlueprintResources/ActorMacros.Switch Has Authority`
    (:`Authority`
      ;[1 1 1] Replicate Physics based Movement from server to the owning client
      (`|ExecutionSequence`
        (:`then_0`
          (`self.ClientSmoothTransform` (`self.GetTransform`) (`GameplayStatics.GetTimeSeconds`)))))
    (:`Remote`
      (set `self.deltaSeconds` DeltaSeconds)
      (if true
        (bind _result (`/Engine/EditorBlueprintResources/StandardMacros.IncrementInt` (`self.ticks`))
          (:`  `
            (set `self.ticks` _result)
            (`KismetSystemLibrary.PrintString` (`KismetStringLibrary.Conv_IntToString` _returnvalue))
            (if (or (> (- _returnvalue (`self.buffersize`)) 0) (>= (`self.ticks`) 3600))
              (`KismetSystemLibrary.PrintString` "skimming###############################" false)
              (set `self.ticks` 0)
              (for _ (range (+ (- _returnvalue 2) 1))
                (`KismetArrayLibrary.Array_Remove` (`self.Transforms`))
                (`KismetArrayLibrary.Array_Remove` (`self.Times`)))
              (`self.K2_SetActorTransform` (`KismetMathLibrary.MakeTransform` (.location (`|GetArrayItem` (`self.Transforms`) 1)) (.rotation (`|GetArrayItem` (`self.Transforms`) 1))) :!label _label)
              (`KismetArrayLibrary.Array_Remove` (`self.Transforms`))
              (`KismetArrayLibrary.Array_Remove` (`self.Times`))
              (set `self.TicksSpentInterpolating` 0)
              (elif (>= _returnvalue 2)
                (if (> _returnvalue_3 1)
                  (`KismetSystemLibrary.PrintString` "interping" false)
                  (`self.K2_SetActorTransform` (`KismetMathLibrary.MakeTransform` (+ (`KismetMathLibrary.VLerp` (.location (`|GetArrayItem` _transforms)) (.location (`|GetArrayItem` _transforms 1)) (/ (`KismetMathLibrary.Conv_IntToDouble` (+ (`self.TicksSpentInterpolating`) 1)) (`KismetMathLibrary.Conv_IntToDouble` _returnvalue_2))) (1.0 0.0 0.0))))
                  (bind _result_2 (`/Engine/EditorBlueprintResources/StandardMacros.IncrementInt` (`self.TicksSpentInterpolating`))
                    (:`  `
                      (set `self.TicksSpentInterpolating` _result_2)
                      (for (_array_element _array_index) _times
                        (if (> _array_index 0)
                          (set `self.InterpTicksNeeded` (+ _interpticksneeded (`KismetMathLibrary.Round` (/ (- _array_element (`|GetArrayItem` _times (- _array_index 1))) (`self.deltaSeconds`)))))))
                      (`KismetSystemLibrary.PrintString` (`KismetStringLibrary.Concat_StrStr` (`KismetStringLibrary.Conv_IntToString` _returnvalue_3) "ticksleft 0f" (`KismetStringLibrary.Conv_IntToString` _returnvalue_2) "Totalticks" (`KismetStringLibrary.Conv_IntToString` _interpticksneeded) "Server Points" (`KismetStringLibrary.Conv_IntToString` (`KismetArrayLibrary.Array_Length` _times))))
                      (set `self.InterpTicksNeeded` 0)))
                  (else
                    (`KismetSystemLibrary.PrintString` "s" false)
                    (goto _label)))
                (else
                  (`KismetSystemLibrary.PrintString` "WAITING FOR SERVER UPDATE!!!!!!!!!!!!!!!!!!!!!!!!" false))))))))))

(fn `UserConstructionScript`)