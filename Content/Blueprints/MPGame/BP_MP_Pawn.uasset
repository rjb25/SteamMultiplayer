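; Multiplayer physics-sphere pawn with server-authoritative movement and a radial blast attack.
; Axis inputs call server events that add linear and angular velocity; clients disable physics at BeginPlay and take the server's transform each Tick, without interpolation.
; ServerBlast applies radial impulses to other pawns and spawns an emitter through ShowBlast.
; The blast trigger and player-start logic are disconnected, so neither runs.
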(event `self.ReceiveBeginPlay`
  ;[1 1 1] Make sure the client isn't doing physics, only the server
  (`/Engine/EditorBlueprintResources/ActorMacros.Switch Has Authority`
    (:`Remote`
      (`PrimitiveComponent.SetSimulatePhysics` (`self.Sphere1`) false))))

(event `ServerMoveForward`
  (params (Value :type "Float (double-precision)"))
  ;[1 1 1] Server-side movement and rotation
  (`/Engine/EditorBlueprintResources/ActorMacros.Switch Has Authority`
    (:`Authority`
      (`PrimitiveComponent.SetAllPhysicsLinearVelocity` (`self.Sphere1`) (* (`self.GetActorForwardVector`) (* Value (`self.MoveForwardScale`))) true))))

(event `InputAxis|LookUp`
  (params (AxisValue :type "Float (single-precision)"))
  ;[1 1 1] Replicate movement inputs from client to server
  (if (!= AxisValue 0.0)
    (`self.ServerLookUp` AxisValue)))

(event `InputAxis|Turn`
  (params (AxisValue :type "Float (single-precision)"))
  ;[1 1 1] Replicate movement inputs from client to server
  (if (!= AxisValue 0.0)
    (`self.ServerTurn` AxisValue)))

(event `ServerMoveRight`
  (params (Value :type "Float (double-precision)"))
  ;[1 1 1] Server-side movement and rotation
  (`/Engine/EditorBlueprintResources/ActorMacros.Switch Has Authority`
    (:`Authority`
      (`PrimitiveComponent.SetAllPhysicsLinearVelocity` (`self.Sphere1`) (* (`self.GetActorRightVector`) (* Value (`self.ActorMoveRightScale`))) true))))

(event `InputAxis|MoveForward`
  (params (AxisValue :type "Float (single-precision)"))
  ;[1 1 1] Replicate movement inputs from client to server
  (if (!= AxisValue 0.0)
    (`self.ServerMoveForward` AxisValue)))

(event `ServerBlast`
  (params (BlastCenter :type "Vector Structure") (BlastPower :type "Float (double-precision)") (BlastRadius :type "Float (double-precision)") (BlastInstigator :type "Pawn Object Reference"))
  ;[0.6959 1 0.7786] Blast attack!
  ;;[1 1 1] Server side handling of the blast attack
  (`|ExecutionSequence`
    (:`then_0`
      (bind _outactors (`GameplayStatics.GetAllActorsOfClass` "BP_MP_Pawn_C"))
      (for _array_element _outactors
        (if (!= _array_element BlastInstigator)
          (bind _asbp_mp_pawn (cast `/Game/Blueprints/MPGame/BP_MP_Pawn` _array_element))
          (`self.GetBlasted` _asbp_mp_pawn BlastCenter BlastPower BlastRadius))))
    (:`then_1`
      (`self.ShowBlast` BlastCenter))))

(event `InputAxis|MoveRight`
  (params (AxisValue :type "Float (single-precision)"))
  ;[1 1 1] Replicate movement inputs from client to server
  (if (!= AxisValue 0.0)
    (`self.ServerMoveRight` AxisValue)))

(event `ServerLookUp`
  (params (Value :type "Float (double-precision)"))
  ;[1 1 1] Server-side movement and rotation
  (`/Engine/EditorBlueprintResources/ActorMacros.Switch Has Authority`
    (:`Authority`
      (`PrimitiveComponent.SetPhysicsAngularVelocityInDegrees` (`self.Sphere1`) (* (`self.GetActorRightVector`) (* Value (`self.LookUpScale`))) true "None"))))

(event `ServerTurn`
  (params (Value :type "Float (double-precision)"))
  ;[1 1 1] Server-side movement and rotation
  (`/Engine/EditorBlueprintResources/ActorMacros.Switch Has Authority`
    (:`Authority`
      (`PrimitiveComponent.SetPhysicsAngularVelocityInDegrees` (`self.Sphere1`) (* (`self.GetActorUpVector`) (* Value (`self.TurnScale`))) true "None"))))

(event `ShowBlast`
  (params (BlastLocation :type "Vector Structure"))
  ;[0.6959 1 0.7786] Blast attack!
  ;;[1 1 1] Spawn the visual effect. Not a reliable function
  (`GameplayStatics.SpawnEmitterAtLocation` (`self.BlastEmitter`) BlastLocation))

(event `self.ReceiveTick`
  (params (DeltaSeconds :type "Float (single-precision)"))
  ;[1 1 1] Replicate Physics based Movement from server to the owning client
  (`/Engine/EditorBlueprintResources/ActorMacros.Switch Has Authority`
    (:`Authority`
      (`self.ClientSmoothTransform` (`self.GetTransform`)))))

(event `ClientSmoothTransform`
  (params (Transform :type "Transform Structure"))
  ;[1 1 1] Replicate Physics based Movement from server to the owning client
  (`self.K2_SetActorTransform` Transform))

(fn `GetBlasted`
  (params (BlastCenter :type "Vector Structure") (BlastPower :type "Float (double-precision)") (BlastRadius :type "Float (double-precision)"))
  (`PrimitiveComponent.AddRadialImpulse` (`self.Sphere1`) BlastCenter BlastRadius BlastPower "RIF_Linear" false))

(fn `SetPlayerStart`)

(fn `UserConstructionScript`
  (`self.SetPlayerStart`))