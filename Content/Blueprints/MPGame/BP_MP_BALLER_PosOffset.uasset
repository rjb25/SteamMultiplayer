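; Multiplayer physics ball pawn that tests hiding latency on the owning client, with simulated packet lag and loss.
; The server alone simulates physics, applying input impulses and sending timestamped transforms every tick.
; The owning client buffers these in time order, interpolates between them and skims the backlog when it grows too large.
; A queued, fading offset from held WASD keys shifts the displayed position to anticipate movement, alongside heavy debug printing.
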(event `self.ReceiveBeginPlay`
  ;[1 1 1] Make sure the client isn't doing physics, only the server
  (`|ExecutionSequence`
    (:`then_0`
      (`KismetSystemLibrary.ExecuteConsoleCommand` "net pktlag=75" null)
      (`KismetSystemLibrary.ExecuteConsoleCommand` "net pktloss=1" null))
    (:`then_1`
      (`/Engine/EditorBlueprintResources/ActorMacros.Switch Has Authority`
        (:`Remote`
          (if (`|EnumEquality` (`self.GetLocalRole`) "ROLE_AutonomousProxy")
            (for _ (range (`self.OffsetQueueLength`))
              (`KismetArrayLibrary.Array_Add` (`self.OffsetQueue`))))
          (`PrimitiveComponent.SetSimulatePhysics` (`self.Ball`) false))))))

(event `ServerMoveForward`
  (params (Value :type "Float (double-precision)"))
  ;[1 1 1] Server-side movement and rotation
  (`/Engine/EditorBlueprintResources/ActorMacros.Switch Has Authority`
    (:`Authority`
      (`PrimitiveComponent.AddImpulse` (`self.Ball`) (`KismetMathLibrary.MakeVector` (* Value (`self.PushForce`))) "None" false))))

(event `ServerMoveRight`
  (params (Value :type "Float (double-precision)"))
  ;[1 1 1] Server-side movement and rotation
  (`/Engine/EditorBlueprintResources/ActorMacros.Switch Has Authority`
    (:`Authority`
      (`PrimitiveComponent.AddImpulse` (`self.Ball`) (`KismetMathLibrary.MakeVector` 0.0 (* Value (`self.PushForce`))) "None" false))))

(event `InputAxis|MoveForward`
  (params (AxisValue :type "Float (single-precision)"))
  ;[1 1 1] Replicate movement inputs from client to server
  (if (!= AxisValue 0.0)
    (`self.ServerMoveForward` AxisValue)))

(event `InputAxis|MoveRight`
  (params (AxisValue :type "Float (single-precision)"))
  ;[1 1 1] Replicate movement inputs from client to server
  (if (!= AxisValue 0.0)
    (`self.ServerMoveRight` AxisValue)))

(event `ClientSmoothTransform`
  (params (Transform :type "Transform Structure") (Time :type "Float (double-precision)"))
  (bind _times (`self.Times`))
  (bind _times_2 (`self.Times`))
  (bind _times_3 (`self.Times`))
  (if (`|EnumEquality` (`self.GetLocalRole`) "ROLE_AutonomousProxy")
    (if (== (`KismetArrayLibrary.Array_Length` _times) 0)
      (`KismetArrayLibrary.Array_Add` (`self.Transforms`) Transform)
      (`KismetArrayLibrary.Array_Add` _times Time)
      (if (and (< (`self.ticks`) 600) (> (`self.ticks`) 300)) :!label _label
        (`KismetSystemLibrary.PrintString` (`KismetStringLibrary.Concat_StrStr` "INSERTED" (`KismetStringLibrary.Conv_DoubleToString` Time)) false true (struct :`G` 0.66 :`B` 1.0 :`A` 1.0) 60.0))
      (elif (> Time (`|GetArrayItem` _times_3))
        (for _index (range (+ (`KismetArrayLibrary.Array_Length` _times_3) 1))
          (if (== _index (`KismetArrayLibrary.Array_LastIndex` _times_2))
            (`KismetArrayLibrary.Array_Add` (`self.Transforms`) Transform)
            (`KismetArrayLibrary.Array_Add` (`self.Times`) Time)
            (break)
            (elif (< Time (`|GetArrayItem` _times_2 _index))
              (`KismetArrayLibrary.Array_Insert` (`self.Transforms`) Transform _index)
              (`KismetArrayLibrary.Array_Insert` _times_2 Time _index)
              (break))))
        (`|ExecutionSequence`
          (:`then_0`
            (`/Engine/EditorBlueprintResources/ActorMacros.Switch Has Authority`
              (:`Remote`
                (bind _outactors (`GameplayStatics.GetAllActorsOfClass` "/Game/Sphere2_Blueprint.Sphere2_Blueprint_C")))))
          (:`then_1`
            (goto _label)))
        (else
          ;[1 1 1] If time is newer than our current interp point
          (`KismetSystemLibrary.PrintString` "1       1        1        1      1      1       1     1 Bad Order"))))))

(event `self.ReceiveTick`
  (params (DeltaSeconds :type "Float (single-precision)"))
  (bind _returnvalue (`GameplayStatics.GetPlayerController` 0))
  (bind _times (`self.Times`))
  (bind _interpticksneeded (`self.InterpTicksNeeded`))
  (bind _ticks (`self.ticks`))
  (bind _transforms (`self.Transforms`))
  (bind _oldestposition (`self.OldestPosition`))
  (bind _transforms_2 (`self.Transforms`))
  (bind _times_2 (`self.Times`))
  (bind _transforms_3 (`self.Transforms`))
  (bind _times_3 (`self.Times`))
  (bind _offsetqueue (`self.OffsetQueue`))
  (bind _offset (`self.Offset`))
  (bind _offsetfadeindex (`self.OffsetFadeIndex`))
  (bind _returnvalue_2 (`KismetArrayLibrary.Array_Length` _transforms))
  (bind _returnvalue_3 (`PlayerController.IsInputKeyDown` _returnvalue "A"))
  (bind _returnvalue_4 (`PlayerController.IsInputKeyDown` _returnvalue "W"))
  (bind _returnvalue_5 (`PlayerController.IsInputKeyDown` _returnvalue "S"))
  (bind _returnvalue_6 (`PlayerController.IsInputKeyDown` _returnvalue "D"))
  (bind _returnvalue_7 (`KismetMathLibrary.Round` (/ (- (`|GetArrayItem` (`self.Times`)) (`self.CurrentTime`)) (`self.deltaSeconds`))))
  (bind _returnvalue_8 (- _returnvalue_7 (`self.TicksSpentInterpolating`)))
  (bind _returnvalue_9 (/ (`KismetMathLibrary.Conv_IntToDouble` (+ (`self.TicksSpentInterpolating`) 1)) (`KismetMathLibrary.Conv_IntToDouble` _returnvalue_7)))
  (`/Engine/EditorBlueprintResources/ActorMacros.Switch Has Authority`
    (:`Authority`
      (`|ExecutionSequence`
        (:`then_0`
          (`self.ClientSmoothTransform` (`self.GetTransform`) (`GameplayStatics.GetTimeSeconds`)))))
    (:`Remote`
      (set `self.deltaSeconds` DeltaSeconds)
      (if (`|EnumEquality` (`self.GetLocalRole`) "ROLE_AutonomousProxy")
        (`|ExecutionSequence`
          (:`then_0`
            (if (and _returnvalue_4 _returnvalue_3)
              (set `self.Offset` (0.7071 -0.7071 0.0))
              (elif (and _returnvalue_6 _returnvalue_4)
                (set `self.Offset` (0.7071 0.7071 0.0))
                (elif (and _returnvalue_5 _returnvalue_6)
                  (set `self.Offset` (-0.7071 0.7071 0.0))
                  (elif (and _returnvalue_3 _returnvalue_5)
                    (set `self.Offset` (-0.7071 -0.7071 0.0))
                    (elif _returnvalue_4
                      (set `self.Offset` (1.0 0.0 0.0))
                      (elif _returnvalue_3
                        (set `self.Offset` (0.0 -1.0 0.0))
                        (elif _returnvalue_5
                          (set `self.Offset` (-1.0 0.0 0.0))
                          (elif _returnvalue_6
                            (set `self.Offset` (0.0 1.0 0.0))
                            (else
                              (set `self.Offset` (0.0 0.0 0.0))))))))))))
          (:`then_1`
            (`KismetArrayLibrary.Array_Remove` _offsetqueue)
            (`KismetArrayLibrary.Array_Add` _offsetqueue)
            (for (_ _array_index) _offsetqueue
              (if (> _array_index _offsetfadeindex)
                (bind _output (`|GetArrayItem` _offsetqueue _array_index))
                (`KismetArrayLibrary.Array_Set` _offsetqueue _array_index (+ _output (/ _offset (`KismetMathLibrary.Conv_IntToDouble` (+ _array_index 1 (* _offsetfadeindex -1))))))
                (else
                  (`KismetArrayLibrary.Array_Set` _offsetqueue _array_index (+ _output _offset))))))
          (:`then_2`
            (bind _result (`/Engine/EditorBlueprintResources/StandardMacros.IncrementInt` (`self.ticks`))
              (:`  `
                (set `self.ticks` _result)
                (if (< _returnvalue_2 5)
                  (`KismetSystemLibrary.PrintString` (`KismetStringLibrary.Conv_IntToString` _returnvalue_2) false))
                (if (or (> (- _returnvalue_2 (`self.buffersize`)) 0) (== (mod _ticks 3600) 0) (== _ticks 60))
                  (`KismetSystemLibrary.PrintString` "skimming###############################")
                  (set `self.last index` (- _returnvalue_2 3))
                  (for _index (range (+ (`self.last index`) 1))
                    (set `self.OldestPosition` (`|GetArrayItem` _transforms_2))
                    (`KismetArrayLibrary.Array_Remove` _transforms_2)
                    (set `self.CurrentTime` (`|GetArrayItem` _times_2))
                    (`KismetArrayLibrary.Array_Remove` _times_2)
                    (if (== _index (`self.last index`))
                      (`KismetSystemLibrary.PrintString` (`KismetStringLibrary.Concat_StrStr` "Reduced to by skimming" (`KismetStringLibrary.Conv_IntToString` (`KismetArrayLibrary.Array_Length` _transforms_2))))))
                  (`self.K2_SetActorTransform` (`KismetMathLibrary.MakeTransform` (+ (.location (`|GetArrayItem` (`self.Transforms`))) (* (`|GetArrayItem` (`self.OffsetQueue`)) (`self.OffsetMult`))) (.rotation (`|GetArrayItem` (`self.Transforms`)))) :!label _label_2)
                  (set `self.OldestPosition` (`|GetArrayItem` _transforms_3))
                  (`KismetArrayLibrary.Array_Remove` _transforms_3)
                  (set `self.CurrentTime` (`|GetArrayItem` _times_3))
                  (`KismetArrayLibrary.Array_Remove` _times_3)
                  (set `self.TicksSpentInterpolating` 0)
                  (if (and (< (`self.ticks`) 600) (> (`self.ticks`) 300))
                    (`KismetSystemLibrary.PrintString` (`KismetStringLibrary.Concat_StrStr` "REMOVED" (`KismetStringLibrary.Conv_DoubleToString` (`self.CurrentTime`))) false true (struct :`G` 0.66 :`B` 1.0 :`A` 1.0) 60.0))
                  (elif (>= _returnvalue_2 1)
                    ;[1 1 1] Replicate Physics based Movement from server to the owning client
                    (if (> _returnvalue_8 1)
                      (`KismetSystemLibrary.PrintString` "interping")
                      (`KismetSystemLibrary.PrintString` (`KismetStringLibrary.Conv_TransformToString` _oldestposition) false)
                      (`self.K2_SetActorTransform` (`KismetMathLibrary.MakeTransform` (+ (`KismetMathLibrary.VLerp` (.location _oldestposition) (.location (`|GetArrayItem` _transforms)) _returnvalue_9) (* (`|GetArrayItem` (`self.OffsetQueue`)) (`self.OffsetMult`))) (`KismetMathLibrary.RInterpTo` (.rotation _oldestposition) (.rotation (`|GetArrayItem` _transforms)) _returnvalue_9 1.0)))
                      (bind _result_2 (`/Engine/EditorBlueprintResources/StandardMacros.IncrementInt` (`self.TicksSpentInterpolating`))
                        (:`  `
                          (set `self.TicksSpentInterpolating` _result_2)
                          (for (_array_element _array_index_2) _times
                            (if (> _array_index_2 0)
                              (set `self.InterpTicksNeeded` (+ _interpticksneeded (`KismetMathLibrary.Round` (/ (- _array_element (`|GetArrayItem` _times (- _array_index_2 1))) (`self.deltaSeconds`)))))))
                          (`KismetSystemLibrary.PrintString` (`KismetStringLibrary.Concat_StrStr` (`KismetStringLibrary.Conv_IntToString` _returnvalue_8) "ticksleft 0f" (`KismetStringLibrary.Conv_IntToString` _returnvalue_7) "Totalticks" (`KismetStringLibrary.Conv_IntToString` _interpticksneeded) "Server Points" (`KismetStringLibrary.Conv_IntToString` (`KismetArrayLibrary.Array_Length` _times))) false)
                          (set `self.InterpTicksNeeded` 0)))
                      (else
                        (`KismetSystemLibrary.PrintString` "s" false)
                        (goto _label_2)))
                    (else
                      (`KismetSystemLibrary.PrintString` "WAITING FOR SERVER UPDATE!!!!!!!!!!!!!!!!!!!!!!!!"))))))))))))

(fn `UserConstructionScript`)