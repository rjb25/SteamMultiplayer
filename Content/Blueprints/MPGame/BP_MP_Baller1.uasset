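; Multiplayer rolling-ball pawn that is server-authoritative, with physics simulation disabled on remote instances.
; Movement axis input calls server events that apply roll torque to the Ball on authority.
; Each server tick calls ClientSmoothTransform, which currently only increments a counter on remotes and applies no transform.
; Remote tick prints and decrements that counter as a call-rate debug readout, and BeginPlay resets simulated packet lag and loss to zero.
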(event `self.ReceiveBeginPlay`
  ;[1 1 1] Make sure the client isn't doing physics, only the server
  (`|ExecutionSequence`
    (:`then_0`
      (`KismetSystemLibrary.ExecuteConsoleCommand` "net pktlag=0" null)
      (`KismetSystemLibrary.ExecuteConsoleCommand` "net pktloss=0" null))
    (:`then_1`
      (`/Engine/EditorBlueprintResources/ActorMacros.Switch Has Authority`
        (:`Remote`
          (`PrimitiveComponent.SetSimulatePhysics` (`self.Ball`) false))))))

(event `ServerMoveForward`
  (params (Value :type "Float (double-precision)"))
  ;[1 1 1] Server-side movement and rotation
  (`/Engine/EditorBlueprintResources/ActorMacros.Switch Has Authority`
    (:`Authority`
      (`PrimitiveComponent.AddTorqueInRadians` (`self.Ball`) (`KismetMathLibrary.MakeVector` 0.0 (* Value (`self.RollTorque`))) "None" false))))

(event `ServerMoveRight`
  (params (Value :type "Float (double-precision)"))
  ;[1 1 1] Server-side movement and rotation
  (`/Engine/EditorBlueprintResources/ActorMacros.Switch Has Authority`
    (:`Authority`
      (`PrimitiveComponent.AddTorqueInRadians` (`self.Ball`) (`KismetMathLibrary.MakeVector` (* Value (`self.RollTorque`) -1.0)) "None" false))))

(event `InputAxis|MoveForward`
  (params (AxisValue :type "Float (single-precision)"))
  ;[1 1 1] Replicate movement inputs from client to server
  (if (!= AxisValue 0.0)
    (`self.ServerMoveForward` AxisValue)))

(event `InputAxis|MoveRight`
  (params (AxisValue :type "Float (single-precision)"))
  ;[1 1 1] Replicate movement inputs from client to server
  (if (!= AxisValue 0.0)
    (`self.ServerMoveRight` AxisValue)))

(event `ClientSmoothTransform`
  (params (Transform :type "Transform Structure") (Time :type "Float (double-precision)"))
  (`/Engine/EditorBlueprintResources/ActorMacros.Switch Has Authority`
    (:`Remote`
      (bind _result (`/Engine/EditorBlueprintResources/StandardMacros.IncrementInt` (`self.ServerCalls`))
        (:`  `
          (set `self.ServerCalls` _result))))))

(event `self.ReceiveTick`
  (params (DeltaSeconds :type "Float (single-precision)"))
  (bind _servercalls (`self.ServerCalls`))
  (`/Engine/EditorBlueprintResources/ActorMacros.Switch Has Authority`
    (:`Authority`
      (`|ExecutionSequence`
        (:`then_0`
          (`self.ClientSmoothTransform` (struct)))))
    (:`Remote`
      (`KismetSystemLibrary.PrintString` (`KismetStringLibrary.Concat_StrStr` (`KismetStringLibrary.Conv_IntToString` _servercalls) "diff" (`KismetStringLibrary.Conv_IntToString` (- _servercalls (`self.RecentCallCount`)))))
      (set `self.RecentCallCount` _servercalls)
      (bind _result (`/Engine/EditorBlueprintResources/StandardMacros.DecrementInt` _servercalls)
        (:`  `
          (set `self.ServerCalls` _result))))))

(fn `UserConstructionScript`)