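; Multiplayer rolling ball pawn that keeps physics simulation on the server and disables it on clients.
; Movement axis inputs pass to server events, which apply roll torque to the Ball.
; Every tick the server sends its transform to the owning client, which snaps to it directly, without interpolation despite the ClientSmoothTransform name.
; Older local torque and velocity nodes remain disconnected.
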(event `self.ReceiveBeginPlay`
  ;[1 1 1] Make sure the client isn't doing physics, only the server
  (`/Engine/EditorBlueprintResources/ActorMacros.Switch Has Authority`
    (:`Remote`
      (`PrimitiveComponent.SetSimulatePhysics` (`self.Ball`) false))))

(event `ServerMoveForward`
  (params (Value :type "Float (double-precision)"))
  ;[1 1 1] Server-side movement and rotation
  (`/Engine/EditorBlueprintResources/ActorMacros.Switch Has Authority`
    (:`Authority`
      (`PrimitiveComponent.AddTorqueInRadians` (`self.Ball`) (`KismetMathLibrary.MakeVector` 0.0 (* Value (`self.RollTorque`))) "None" false))))

(event `ServerMoveRight`
  (params (Value :type "Float (double-precision)"))
  ;[1 1 1] Server-side movement and rotation
  (`/Engine/EditorBlueprintResources/ActorMacros.Switch Has Authority`
    (:`Authority`
      (`PrimitiveComponent.AddTorqueInRadians` (`self.Ball`) (`KismetMathLibrary.MakeVector` (* Value (`self.RollTorque`) -1.0)) "None" false))))

(event `InputAxis|MoveForward`
  (params (AxisValue :type "Float (single-precision)"))
  ;[1 1 1] Replicate movement inputs from client to server
  (if (!= AxisValue 0.0)
    (`self.ServerMoveForward` AxisValue)))

(event `InputAxis|MoveRight`
  (params (AxisValue :type "Float (single-precision)"))
  ;[1 1 1] Replicate movement inputs from client to server
  (if (!= AxisValue 0.0)
    (`self.ServerMoveRight` AxisValue)))

(event `InputAxis|MoveRight`
  (params (AxisValue :type "Float (single-precision)"))
  ;[1 1 1] Roll left/right
)

(event `InputAxis|MoveForward`
  (params (AxisValue :type "Float (single-precision)"))
  ;[1 1 1] Roll forwards/backwards
)

(event `self.ReceiveTick`
  (params (DeltaSeconds :type "Float (single-precision)"))
  ;[1 1 1] Replicate Physics based Movement from server to the owning client
  (`/Engine/EditorBlueprintResources/ActorMacros.Switch Has Authority`
    (:`Authority`
      (`self.ClientSmoothTransform` (`self.GetTransform`)))))

(event `ClientSmoothTransform`
  (params (Transform :type "Transform Structure"))
  ;[1 1 1] Replicate Physics based Movement from server to the owning client
  (`/Engine/EditorBlueprintResources/ActorMacros.Switch Has Authority`
    (:`Remote`
      (`self.K2_SetActorTransform` (`KismetMathLibrary.MakeTransform` (.location Transform) (.rotation Transform) (.scale Transform))))))

(fn `UserConstructionScript`)