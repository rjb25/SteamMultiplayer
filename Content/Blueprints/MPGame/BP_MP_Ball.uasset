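; BP_MP_Ball is a multiplayer, input-driven physics ball that can be knocked around by radial blast impulses.
; Movement input goes through server events that add linear velocity to the sphere, with physics simulation disabled on clients.
; Each tick the server passes its transform to ClientSmoothTransform, which sets it directly without interpolation.
; The construction script calls SetPlayerStart, whose game-mode spawn logic is disconnected.
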(event `self.ReceiveBeginPlay`
  ;[1 1 1] Make sure the client isn't doing physics, only the server
  (`/Engine/EditorBlueprintResources/ActorMacros.Switch Has Authority`
    (:`Remote`
      (`PrimitiveComponent.SetSimulatePhysics` (`self.Sphere1`) false))))

(event `ServerMoveForward`
  (params (Value :type "Float (double-precision)"))
  ;[1 1 1] Server-side movement and rotation
  (`/Engine/EditorBlueprintResources/ActorMacros.Switch Has Authority`
    (:`Authority`
      (`PrimitiveComponent.SetAllPhysicsLinearVelocity` (`self.Sphere1`) (* (`self.GetActorForwardVector`) (* Value (`self.MoveForwardScale`))) true))))

(event `ServerMoveRight`
  (params (Value :type "Float (double-precision)"))
  ;[1 1 1] Server-side movement and rotation
  (`/Engine/EditorBlueprintResources/ActorMacros.Switch Has Authority`
    (:`Authority`
      (`PrimitiveComponent.SetAllPhysicsLinearVelocity` (`self.Sphere1`) (* (`self.GetActorRightVector`) (* Value (`self.ActorMoveRightScale`))) true))))

(event `InputAxis|MoveForward`
  (params (AxisValue :type "Float (single-precision)"))
  ;[1 1 1] Replicate movement inputs from client to server
  (if (!= AxisValue 0.0)
    (`self.ServerMoveForward` AxisValue)))

(event `InputAxis|MoveRight`
  (params (AxisValue :type "Float (single-precision)"))
  ;[1 1 1] Replicate movement inputs from client to server
  (if (!= AxisValue 0.0)
    (`self.ServerMoveRight` AxisValue)))

(event `self.ReceiveTick`
  (params (DeltaSeconds :type "Float (single-precision)"))
  ;[1 1 1] Replicate Physics based Movement from server to the owning client
  (`/Engine/EditorBlueprintResources/ActorMacros.Switch Has Authority`
    (:`Authority`
      (`self.ClientSmoothTransform` (`self.GetTransform`)))))

(event `ClientSmoothTransform`
  (params (Transform :type "Transform Structure"))
  ;[1 1 1] Replicate Physics based Movement from server to the owning client
  (`self.K2_SetActorTransform` Transform))

(fn `GetBlasted`
  (params (BlastCenter :type "Vector Structure") (BlastPower :type "Float (double-precision)") (BlastRadius :type "Float (double-precision)"))
  (`PrimitiveComponent.AddRadialImpulse` (`self.Sphere1`) BlastCenter BlastRadius BlastPower "RIF_Linear" false))

(fn `SetPlayerStart`)

(fn `UserConstructionScript`
  (`self.SetPlayerStart`))